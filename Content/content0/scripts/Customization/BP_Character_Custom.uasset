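; Customizable character actor that shows the player's chosen head and spine items and outfit colors, with hooks for turning, hat selection and intro scenes.
; Item meshes and transforms come from data table rows named in the GameInstance, though material assignment is disconnected.
; GameInstance color, brightness and saturation values feed custom primitive data on the items, shirt and shorts.
; Events set pose flags, fade an animation-strength float by timeline, and hold the transform across a tick.
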(event `Turn 180`
  (set `self.Turn To 180?` true)
  (set `self.Turn To Default?` false))

(event `Turn To Default`
  (set `self.Turn To Default?` true)
  (set `self.Turn To 180?` false))

(event `Hat Select`
  (set `self.Hat Selected?` true))

(event `Hat Deselect`
  (set `self.Hat Selected?` false))

(event `Get Head Info`
  (bind _returnvalue (`|GetDataTableRow` "/Game/content0/Customization_Comunication/DT_Custom_Head.DT_Custom_Head" (`/Game/content0/scripts/base/myGameInstance.Head Row Name` (`/Game/content0/scripts/base/myFunctions.Get GInstance`)))
    (:`then`
      (bind (_staticmesh _materialslot1 _materialslot2 _meshoffsetrotationscale) (break `/Game/content0/Customization_Comunication/STR_Customization` _returnvalue))
      (bind _output_get (set `self.Head Struct` (make `/Game/content0/worlds/main_menu_new/ui/Customization/Comunication/STR_Item_Data` _staticmesh _materialslot1 _materialslot2 _meshoffsetrotationscale)))
      (bind (_staticmesh_2 _materialslot1_2 _materialslot2_2 _transform) (break `/Game/content0/worlds/main_menu_new/ui/Customization/Comunication/STR_Item_Data` _output_get))
      (`/Engine/EditorBlueprintResources/StandardMacros.IsValid` _staticmesh_2
        (:`Is Valid`
          (`StaticMeshComponent.SetStaticMesh` (`self.StaticMesh`) _staticmesh_2)
          (`SceneComponent.K2_SetRelativeTransform` (`self.StaticMesh`) _transform false false))
        (:`Is Not Valid`
          (`StaticMeshComponent.SetStaticMesh` (`self.StaticMesh`) null))))))

(event `Get Spine Info`
  (bind _returnvalue (`|GetDataTableRow` "/Game/content0/Customization_Comunication/DT_Custom_Spine.DT_Custom_Spine" (`/Game/content0/scripts/base/myGameInstance.Spine Row Name` (`/Game/content0/scripts/base/myFunctions.Get GInstance`)))
    (:`then`
      (bind (_staticmesh _materialslot1 _materialslot2 _meshoffsetrotationscale) (break `/Game/content0/Customization_Comunication/STR_Customization` _returnvalue))
      (bind _output_get (set `self.Spine Struct` (make `/Game/content0/worlds/main_menu_new/ui/Customization/Comunication/STR_Item_Data` _staticmesh _materialslot1 _materialslot2 _meshoffsetrotationscale)))
      (bind (_staticmesh_2 _materialslot1_2 _materialslot2_2 _transform) (break `/Game/content0/worlds/main_menu_new/ui/Customization/Comunication/STR_Item_Data` _output_get))
      (`/Engine/EditorBlueprintResources/StandardMacros.IsValid` _staticmesh_2
        (:`Is Valid`
          (`StaticMeshComponent.SetStaticMesh` (`self.Spine Mesh`) _staticmesh_2)
          (`SceneComponent.K2_SetRelativeTransform` (`self.Spine Mesh`) _transform false false))
        (:`Is Not Valid`
          (`StaticMeshComponent.SetStaticMesh` (`self.Spine Mesh`) null))))))

(event `Change Color Head`
  (bind _returnvalue (`/Game/content0/scripts/base/myFunctions.Get GInstance`))
  (`PrimitiveComponent.SetDefaultCustomPrimitiveDataFloat` (`self.StaticMesh`) 0 (`/Game/content0/scripts/base/myGameInstance.Head Color` _returnvalue))
  (`PrimitiveComponent.SetDefaultCustomPrimitiveDataFloat` (`self.StaticMesh`) 1 (`/Game/content0/scripts/base/myGameInstance.Head Brithness` _returnvalue))
  (`PrimitiveComponent.SetDefaultCustomPrimitiveDataFloat` (`self.StaticMesh`) 2 (`/Game/content0/scripts/base/myGameInstance.Head Saturation` (`/Game/content0/scripts/base/myFunctions.Get GInstance`))))

(event `Change Spine Color`
  (bind _returnvalue (`/Game/content0/scripts/base/myFunctions.Get GInstance`))
  (bind _spine_mesh (`self.Spine Mesh`))
  (`PrimitiveComponent.SetDefaultCustomPrimitiveDataFloat` (`self.Spine Mesh`) 0 (`/Game/content0/scripts/base/myGameInstance.Spine Color` (`/Game/content0/scripts/base/myFunctions.Get GInstance`)))
  (`PrimitiveComponent.SetDefaultCustomPrimitiveDataFloat` _spine_mesh 1 (`/Game/content0/scripts/base/myGameInstance.Spine Brithness` _returnvalue))
  (`PrimitiveComponent.SetDefaultCustomPrimitiveDataFloat` _spine_mesh 2 (`/Game/content0/scripts/base/myGameInstance.Spine Saturation` _returnvalue)))

(event `self.ReceiveBeginPlay`
  (`self.Get Head Info`)
  (`self.Get Spine Info`)
  (`self.Change Color Head`)
  (`self.Change Spine Color`)
  (`self.Change Color Shirt`)
  (`self.Change Color Shorts`))

(event `Change Color Shirt`
  (bind _returnvalue (`/Game/content0/scripts/base/myFunctions.Get GInstance`))
  ; Shorts + Shirt
  (`PrimitiveComponent.SetDefaultCustomPrimitiveDataFloat` (`self.stylized_man`) 0 (`/Game/content0/scripts/base/myGameInstance.Color Shirt` _returnvalue))
  (`PrimitiveComponent.SetDefaultCustomPrimitiveDataFloat` (`self.stylized_man`) 1 (`/Game/content0/scripts/base/myGameInstance.Brithness Shirt` _returnvalue))
  (`PrimitiveComponent.SetDefaultCustomPrimitiveDataFloat` (`self.stylized_man`) 4 (`/Game/content0/scripts/base/myGameInstance.Shirt Saturation` _returnvalue)))

(event `Change Color Shorts`
  (bind _returnvalue (`/Game/content0/scripts/base/myFunctions.Get GInstance`))
  ; Shorts + Shirt
  (`PrimitiveComponent.SetDefaultCustomPrimitiveDataFloat` (`self.stylized_man`) 2 (`/Game/content0/scripts/base/myGameInstance.Color Shorts` _returnvalue))
  (`PrimitiveComponent.SetDefaultCustomPrimitiveDataFloat` (`self.stylized_man`) 3 (`/Game/content0/scripts/base/myGameInstance.Brithness Shorts` _returnvalue))
  (`PrimitiveComponent.SetDefaultCustomPrimitiveDataFloat` (`self.stylized_man`) 5 (`/Game/content0/scripts/base/myGameInstance.Shorts Saturation` (`/Game/content0/scripts/base/myFunctions.Get GInstance`))))

(event `Animation Blueprint Lerp`
  ; Scenes Intro
  (`TimelineComponent.SetPlayRate` (`self.Timeline`) 2.0)
  (bind (_direction _newtrack_0) (`Timeline|Timeline` :!via `PlayFromStart` :!label _label)
    (:`Update`
      (set `self.Animation Blueprint Strenght` _newtrack_0))))

(event `Animation Bp Unlerp`
  ; Scenes Intro
  (goto _label :!via `ReverseFromEnd`))

(event `Keep Transform State`
  ; Scenes Intro
  (bind _output_get (set `self.Transform After Sequnce` (`self.GetTransform`)))
  (`KismetSystemLibrary.DelayUntilNextTick`)
  (`self.K2_SetActorTransform` _output_get))

(fn `UserConstructionScript`)