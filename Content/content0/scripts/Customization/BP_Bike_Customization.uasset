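; Bike actor for customization that shows the player's chosen paint color and brightness.
; It writes both values from the game instance into the Bike component's custom primitive data on BeginPlay, with separate events to reapply each one.
; KeepTransformState caches the actor transform, apparently around a sequence, but the logic that would restore it is disconnected and never runs.
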(event `Keep Transform State`
  (bind _output_get (set `self.Transform After Sequnce` (`self.GetTransform`)))
  (`KismetSystemLibrary.DelayUntilNextTick`))

(event `self.ReceiveBeginPlay`
  (bind _returnvalue (`/Game/content0/scripts/base/myFunctions.Get GInstance`))
  (`PrimitiveComponent.SetDefaultCustomPrimitiveDataFloat` (`self.bike`) 0 (`/Game/content0/scripts/base/myGameInstance.Bike Color` _returnvalue))
  (`PrimitiveComponent.SetDefaultCustomPrimitiveDataFloat` (`self.bike`) 1 (`/Game/content0/scripts/base/myGameInstance.Bike Brithness` _returnvalue)))

(event `Change Color`
  (`PrimitiveComponent.SetDefaultCustomPrimitiveDataFloat` (`self.bike`) 0 (`/Game/content0/scripts/base/myGameInstance.Bike Color` (`/Game/content0/scripts/base/myFunctions.Get GInstance`))))

(event `Change Brithness`
  (`PrimitiveComponent.SetDefaultCustomPrimitiveDataFloat` (`self.bike`) 1 (`/Game/content0/scripts/base/myGameInstance.Bike Brithness` (`/Game/content0/scripts/base/myFunctions.Get GInstance`))))

(fn `UserConstructionScript`)